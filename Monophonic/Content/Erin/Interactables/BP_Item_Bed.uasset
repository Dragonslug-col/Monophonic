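; Interactable bed item that ends the night and starts the next day.
; On Interact, it acts only if the MonoGameInstance Night flag is set, then clears that flag.
; It then increments DayCount and resets ChoreCount on the BP_FirstPersonCharacter of player 0.
; A trailing cast of BP_MasterItem to Actor has nothing after it.
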(event EventBeginPlay
  (|CallParentFunction) ; This node is disabled and will not be called.\nDrag off pins to build functionality.
)

(event Collision|EventActorBeginOverlap
  (params (OtherActor :type Actor%20Object%20Reference)))

(event EventInteract
  (if true
    (bind _asmono_game_instance (Utilities|Casting|CastToMonoGameInstance (Game|GetGameInstance)))
    (if (Variables|/Game/Erin/MonoGameInstance.MonoGameInstance_C|GetNight? _asmono_game_instance)
      (bind _asmono_game_instance_2 (Utilities|Casting|CastToMonoGameInstance (Game|GetGameInstance)))
      (Variables|/Game/Erin/MonoGameInstance.MonoGameInstance_C|SetNight? _asmono_game_instance_2 false)
      (bind _asbp_first_person_character (Utilities|Casting|CastToBP_FirstPersonCharacter (Game|GetPlayerCharacter 0)))
      (Variables|/Game/FirstPerson/Blueprints/BP_FirstPersonCharacter.BP_FirstPersonCharacter_C|SetDayCount _asbp_first_person_character (+ (Variables|/Game/FirstPerson/Blueprints/BP_FirstPersonCharacter.BP_FirstPersonCharacter_C|GetDayCount _asbp_first_person_character) 1))
      (Variables|/Game/FirstPerson/Blueprints/BP_FirstPersonCharacter.BP_FirstPersonCharacter_C|SetChoreCount _asbp_first_person_character 0)
      (Utilities|Casting|CastToActorClass "/Game/Erin/Interactables/BP_MasterItem.BP_MasterItem_C"))))

(fn ConstructionScript
  (|CallParentFunction))