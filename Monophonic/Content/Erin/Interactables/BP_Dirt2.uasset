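; BP_Dirt2 is an interactable dirt chore that the player cleans while holding a specific item.
; Interacting with that item swaps the mesh to the cleaned material, completes the chore and updates the linked job list actors; otherwise the HUD plays its DirtTalk animation.
; A short Delayed flag debounces interaction.
; Tick polls the player's DayChange flag to restore the mud material and make the chore available again.
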(event Collision|EventActorBeginOverlap
  (params (OtherActor :type Actor%20Object%20Reference)))

(event EventTick
  (params (DeltaSeconds :type Float%20%28single-precision%29))
  (bind _asbp_first_person_character (Utilities|Casting|CastToBP_FirstPersonCharacter (Game|GetPlayerCharacter 0)))
  (if (Variables|/Game/FirstPerson/Blueprints/BP_FirstPersonCharacter.BP_FirstPersonCharacter_C|GetDayChange? _asbp_first_person_character)
    (Utilities|FlowControl|Delay 0.1)
    (Variables|Default|SetCompleted? false)
    (Rendering|Material|SetMaterial (Variables|Default|GetStaticMesh) 0 "/Game/Erin/MudTextures/Mud2Files/Mud2.Mud2")))

(event EventInteract
  (if (not (Variables|Default|GetDelayed))
    (bind _returnvalue (Actor|GetActorOfClass "/Game/FirstPerson/Blueprints/BP_FirstPersonCharacter.BP_FirstPersonCharacter_C"))
    (if (not (Variables|Default|GetCompleted?))
      (if (Utilities|Enum|Equal(Enum) (Variables|/Game/FirstPerson/Blueprints/BP_FirstPersonCharacter.BP_FirstPersonCharacter_C|GetHeldItemEnum _returnvalue) "NewEnumerator1")
        (Rendering|Material|SetMaterial (Variables|Default|GetStaticMesh) 0 "/Game/Erin/MudTextures/Cleaned.Cleaned")
        (CallFunction|ChoreCompleted)
        (Variables|Default|SetCompleted? true)
        (for _array_element (Variables|Default|GetJoblistactorRef)
          (Default|UpdateJob _array_element)
          (Variables|Default|SetDelayed true)
          (Utilities|FlowControl|Delay 0.2)
          (Variables|Default|SetDelayed false))
        (else
          (bind _asbp_first_person_character (Utilities|Casting|CastToBP_FirstPersonCharacter (Game|GetPlayerCharacter 0)))
          (UserInterface|Animation|PlayAnimation (Variables|/Game/FirstPerson/Blueprints/BP_FirstPersonCharacter.BP_FirstPersonCharacter_C|GetHUD _asbp_first_person_character) (Variables|/Game/Erin/HUD/UI_HUD.UI_HUD_C|GetDirtTalk (Variables|/Game/FirstPerson/Blueprints/BP_FirstPersonCharacter.BP_FirstPersonCharacter_C|GetHUD _asbp_first_person_character)) 0.0 1 "Forward" 1.0 false)
          (Variables|Default|SetDelayed true)
          (Utilities|FlowControl|Delay 0.2)
          (Variables|Default|SetDelayed false))))))

(event EventBeginPlay
  (bind _asui_interact (Utilities|Casting|CastToUI_Interact (UserInterface|GetWidget (Variables|Default|GetWidget))))
  (Variables|Default|SetInteractionWidget _asui_interact))

(fn ConstructionScript
  (|CallParentFunction))