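; BP_Item_Plant is an interactable plant that serves as a repeatable daily chore for the first-person player.
; Interacting while holding the required item swaps the mesh to a grass material, marks the chore completed and updates each referenced job list actor.
; Tick polls the player's DayChange flag to clear completion and restore the dark material, with a leftover debug print.
; BeginPlay caches the widget component's UI_Interact as the interaction widget.
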(event Collision|EventActorBeginOverlap
  (params (OtherActor :type Actor%20Object%20Reference)))

(event EventTick
  (params (DeltaSeconds :type Float%20%28single-precision%29))
  (Utilities|FlowControl|Sequence
    (:then_0
      (bind _asbp_first_person_character (Utilities|Casting|CastToBP_FirstPersonCharacter (Game|GetPlayerCharacter 0)))
      (if (Variables|/Game/FirstPerson/Blueprints/BP_FirstPersonCharacter.BP_FirstPersonCharacter_C|GetDayChange? _asbp_first_person_character)
        (Variables|Default|SetCompleted? false)
        (Rendering|Material|SetMaterial (Variables|Default|GetStaticMesh) 0 "/Game/Erin/DarkMat.DarkMat")
        (Development|PrintString "Hello")))))

(event EventInteract
  (bind _returnvalue (Actor|GetActorOfClass "/Game/FirstPerson/Blueprints/BP_FirstPersonCharacter.BP_FirstPersonCharacter_C"))
  (if (Utilities|Enum|Equal(Enum) (Variables|/Game/FirstPerson/Blueprints/BP_FirstPersonCharacter.BP_FirstPersonCharacter_C|GetHeldItemEnum _returnvalue) "NewEnumerator0")
    (if (not (Variables|Default|GetCompleted?))
      (Rendering|Material|SetMaterial (Variables|Default|GetStaticMesh) 0 "/Game/StarterContent/Materials/M_Ground_Grass.M_Ground_Grass")
      (CallFunction|ChoreCompleted)
      (Variables|Default|SetCompleted? true)
      (for _array_element (Variables|Default|GetJoblistactorRef)
        (Default|UpdateJob _array_element)))))

(event EventBeginPlay
  (Utilities|FlowControl|Sequence
    (:then_0
      (bind _asui_interact (Utilities|Casting|CastToUI_Interact (UserInterface|GetWidget (Variables|Default|GetWidget))))
      (Variables|Default|SetInteractionWidget _asui_interact))))

(fn ConstructionScript
  (|CallParentFunction))