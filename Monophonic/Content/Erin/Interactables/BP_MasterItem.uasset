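; Interactable item, apparently a base by its name, that the first-person character can pick up and that can report completed chores.
; While traces keep hitting it and CanInteract is set, it shows an animated prompt widget and outline overlay, cleared by a short retriggerable delay.
; If the player's hands are free, pickup passes its mesh, item and class to the character, then destroys the actor.
; ChoreCompleted increments the character's chore count.
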(event Custom|PickUpEvent
  (params (Item :type HeldItemEnum%20Enum :default "NewEnumerator3"))
  (bind _returnvalue (Actor|GetActorOfClass "/Game/FirstPerson/Blueprints/BP_FirstPersonCharacter.BP_FirstPersonCharacter_C"))
  (if (not (Variables|/Game/FirstPerson/Blueprints/BP_FirstPersonCharacter.BP_FirstPersonCharacter_C|GetIsHolding? _returnvalue))
    (Default|RecPickUp _returnvalue (Variables|/Script/Engine.StaticMeshComponent|GetStaticMesh (Variables|Default|GetStaticMesh)) Item (Utilities|GetClass self))
    (Actor|DestroyActor)))

(event Custom|ChoreCompleted
  (bind _asbp_first_person_character (Utilities|Casting|CastToBP_FirstPersonCharacter (Game|GetPlayerCharacter 0)))
  (Variables|/Game/FirstPerson/Blueprints/BP_FirstPersonCharacter.BP_FirstPersonCharacter_C|SetChoreCount _asbp_first_person_character (+ (Variables|/Game/FirstPerson/Blueprints/BP_FirstPersonCharacter.BP_FirstPersonCharacter_C|GetChoreCount _asbp_first_person_character) 1)))

(event EventBeginPlay
  (bind _asui_interact (Utilities|Casting|CastToUI_Interact (UserInterface|GetWidget (Variables|Default|GetWidget))))
  (Variables|Default|SetInteractionWidget _asui_interact))

(event EventCanReceiveTrace
  (params (CanInteract :type Boolean))
  (bind _interactionwidget (Variables|Default|GetInteractionWidget))
  (if (Variables|Default|GetCanInteract)
    (Rendering|SetVisibility (Variables|Default|GetWidget) true false)
    (Rendering|Material|SetOverlayMaterial (Variables|Default|GetStaticMesh) "/Game/Erin/InteractiveSystem/Outline.Outline" :!class /Script/Engine.MeshComponent)
    (UserInterface|Animation|PlayAnimation _interactionwidget (Variables|/Game/Erin/InteractiveSystem/UI_Interact.UI_Interact_C|GetPopUp _interactionwidget) 0.0 1 "Reverse" 1.5 false)
    (Utilities|FlowControl|RetriggerableDelay 0.1)
    (Rendering|SetVisibility (Variables|Default|GetWidget) false false)
    (Rendering|Material|SetOverlayMaterial (Variables|Default|GetStaticMesh) 0 :!class /Script/Engine.MeshComponent)))

(fn ConstructionScript)